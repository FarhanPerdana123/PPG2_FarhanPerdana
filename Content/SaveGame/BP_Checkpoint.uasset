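; BP_Checkpoint is an interactable save point that records the player's data through the game instance.
; Its sphere overlap stores any actor implementing BPI_Player as the overlapped actor.
; On Interact, it pulls that actor's player data via the interface, saves it synchronously through a game instance message, and prints the saved player transform.
; The stored reference is never cleared when the overlap ends.
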(event OnComponentBeginOverlap(Sphere)
  (params (OverlappedComponent :type Primitive%20Component%20Object%20Reference) (OtherActor :type Actor%20Object%20Reference) (OtherComp :type Primitive%20Component%20Object%20Reference) (OtherBodyIndex :type Integer) (bFromSweep :type Boolean) (SweepResult :type Hit%20Result%20Structure%20%28by%20ref%29))
  (if (Utilities|DoesObjectImplementInterface OtherActor "/Game/ThirdPerson/Blueprints/BPI_Player.BPI_Player_C")
    (Variables|Default|SetOverlappedActor OtherActor)))

(event EventBeginPlay)

(event Collision|EventActorBeginOverlap
  (params (OtherActor :type Actor%20Object%20Reference)))

(event EventTick
  (params (DeltaSeconds :type Float%20%28single-precision%29)))

(event EventInteract
  (bind _overlappedactor (Variables|Default|GetOverlappedActor))
  (if (Utilities|DoesObjectImplementInterface _overlappedactor "/Game/ThirdPerson/Blueprints/BPI_Player.BPI_Player_C")
    (bind _savegamedata (Class|BPIPlayer|GetPlayerData(Message) _overlappedactor))
    (Class|BPISave|SavePlayer(Message) (Game|GetGameInstance) false _savegamedata)
    (Development|PrintString (Utilities|String|ToString(Transform) (Utilities|Struct|BreakS_PlayerData _savegamedata)))))

(fn ConstructionScript)